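; AutoMortar_BP is an automated mortar actor that sets up its aiming and health bar when play begins.
; On BeginPlay it initialises the TankAiming component with its Barrel and Dome, the Dome acting as turret.
; It then casts the HealthBarWidget component's user widget to HealthBar and hands it a self reference.
; Tick, overlap and construction logic are empty, so this graph contains only startup wiring.
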(event EventBeginPlay
  (Class|TankAimingComponent|Initialise (Variables|Default|GetTankAiming) (Variables|Default|GetBarrel) (Variables|Default|GetDome))
  (CallFunction|InitialiseHealthBarWidget))

(event Collision|EventActorBeginOverlap
  (params (OtherActor :type Actor%20Object%20Reference)))

(event EventTick
  (params (DeltaSeconds :type Float%20%28single-precision%29)))

(fn ConstructionScript)

(fn InitialiseHealthBarWidget
  (bind _ashealth_bar (Utilities|Casting|CastToHealthBar (UserInterface|GetUserWidgetObject (Variables|Default|GetHealth%20Bar%20Widget))))
  (Variables|/Game/UI/HealthBar.HealthBar_C|SetMortarBP_Reference _ashealth_bar self)
  (return))